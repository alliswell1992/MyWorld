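; BP_ClimateController runs a looping seasonal cycle that drives global environment material parameters.
; A BeginPlay delay loop sets autumn, snow, spring and leaf-fall targets plus a season index.
; Tick passes targets to a macro that steps MP_Globle scalars outside a dead band, signed current-minus-target, so away from target as wired.
; Tick also lerps the season value, but its ambient audio cue update is never run.
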(event `self.ReceiveBeginPlay`
  (`KismetSystemLibrary.Delay` 5.0)
  (set `self.AutumnTarget` 1.0 :!label _label)
  (set `self.TargetSeasonValue` 1.0)
  (`KismetSystemLibrary.Delay` 25.0)
  (set `self.LeaveFallTarget` 5.0)
  (set `self.AutumnTarget` 0.0)
  (`KismetSystemLibrary.Delay` 5.0)
  (set `self.SnowTarget` 4.0)
  (set `self.TargetSeasonValue` 2.0)
  (`KismetSystemLibrary.Delay` 25.0)
  (set `self.SnowTarget` 0.0)
  (set `self.SpringTarget` 1.0)
  (set `self.TargetSeasonValue` 3.0)
  (set `self.LeaveFallTarget` 0.0)
  (`KismetSystemLibrary.Delay` 10.0)
  (set `self.CurrentSeasonValue` 0.0)
  (set `self.TargetSeasonValue` 0.0)
  (set `self.SpringTarget` 0.0)
  (`KismetSystemLibrary.Delay` 20.0)
  (goto _label))

(event `self.ReceiveTick`
  (params (DeltaSeconds :type "Float (single-precision)"))
  (`self.ParameterUpdate M` (`self.AutumnTarget`) "Autum"
    (:`OutputPin`
      (`self.ParameterUpdate M` (`self.SnowTarget`) "SnowBias"
        (:`OutputPin`
          (`self.ParameterUpdate M` (`self.SpringTarget`) "Spring"
            (:`OutputPin`
              (`self.ParameterUpdate M` (`self.LeaveFallTarget`) "LeaveFall"
                (:`OutputPin`
                  (bind _output_get (set `self.CurrentSeasonValue` (mod (`KismetMathLibrary.Lerp` (`self.CurrentSeasonValue`) (`self.TargetSeasonValue`) 0.01) 4.0))))))))))))

(fn `UserConstructionScript`)