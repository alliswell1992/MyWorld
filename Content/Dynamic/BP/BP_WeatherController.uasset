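; Weather controller that plays a timed sequence: clouds and gloom targets change, rain starts, then stops and the targets change again.
; BeginPlay attaches the Niagara rain to the player controller's root; ToggleRain switches it and rain playback, flipping the step sign.
; Tick steps sky cloud opacity and MP_Globle's Gloom and Rain Level by fixed increments, then updates the sky.
; Rain Level compares against TargetCloudOpacity, leaving TargetRainLevel unread.
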(event `self.ReceiveBeginPlay`
  (`KismetSystemLibrary.Delay` 0.2)
  (`SceneComponent.K2_AttachToComponent` (`self.Nig_rain`) (`Actor.RootComponent` (`GameplayStatics.GetPlayerController` 0)) "None" "SnapToTarget" "SnapToTarget" "SnapToTarget" true)
  (`KismetSystemLibrary.Delay` 5.0)
  (set `self.TargetCloudOpacity` 5.0)
  (set `self.TargetGloomLevel` 0.1)
  (`KismetSystemLibrary.Delay` 20.0)
  (`self.Toggle Rain` true)
  (`KismetSystemLibrary.Delay` 30.0)
  (`self.Toggle Rain` false)
  (set `self.TargetCloudOpacity` 0.7)
  (set `self.TargetGloomLevel` 1.0))

(event `self.ReceiveTick`
  (params (DeltaSeconds :type "Float (single-precision)"))
  (bind _cloud_opacity (`/Engine/EngineSky/BP_Sky_Sphere.Cloud opacity` (`self.Sky`)))
  (bind _returnvalue (- (`self.TargetCloudOpacity`) _cloud_opacity))
  (bind _returnvalue_2 (`KismetMaterialLibrary.GetScalarParameterValue` "/Game/Dynamic/Materials/MP_Globle.MP_Globle" "Gloom"))
  (bind _returnvalue_3 (- (`self.TargetGloomLevel`) _returnvalue_2))
  (if (> (`KismetMathLibrary.Abs` _returnvalue_3) 0.1)
    (`KismetMaterialLibrary.SetScalarParameterValue` "/Game/Dynamic/Materials/MP_Globle.MP_Globle" "Gloom" (+ _returnvalue_2 (* (`self.Change Scale`) (select `bool` (> _returnvalue_3 0.0) :`false` 1.0 :`true` -1.0 :!type "Float (single-precision)")))))
  (if (> (`KismetMathLibrary.Abs` _returnvalue) 0.1)
    (set `/Engine/EngineSky/BP_Sky_Sphere.Cloud opacity` (+ _cloud_opacity (* (`self.Change Scale`) (select `bool` (> _returnvalue 0.0) :`false` 1.0 :`true` -1.0 :!type "Float (single-precision)"))) (`self.Sky`)))
  (bind _returnvalue_4 (`KismetMaterialLibrary.GetScalarParameterValue` "/Game/Dynamic/Materials/MP_Globle.MP_Globle" "Rain Level"))
  (bind _returnvalue_5 (- (`self.TargetCloudOpacity`) _returnvalue_4))
  (if (> (`KismetMathLibrary.Abs` _returnvalue_5) 0.1)
    (`KismetMaterialLibrary.SetScalarParameterValue` "/Game/Dynamic/Materials/MP_Globle.MP_Globle" "Rain Level" (+ _returnvalue_4 (* (`self.Change Scale`) (select `bool` (> _returnvalue_5 0.0) :`false` 1.0 :`true` -1.0 :!type "Float (single-precision)")))))
  (`/Engine/EngineSky/BP_Sky_Sphere.UpdateSky` (`self.Sky`)))

(event `Toggle Rain`
  (params (Enable :type Boolean))
  (if Enable
    (`ActorComponent.SetActive` (`self.Nig_rain`) true false)
    (`AudioComponent.Play` (`self.Rain`) 0.0)
    (set `self.Change Scale` 0.1)
    (`self.SetActorTickEnabled` true)
    (set `self.TargetRainLevel` 0.9)
    (else
      (`ActorComponent.SetActive` (`self.Nig_rain`) false false)
      (`AudioComponent.Stop` (`self.Rain`))
      (set `self.Change Scale` -0.1)
      (`self.SetActorTickEnabled` true)
      (set `self.TargetRainLevel` 0.0))))

(fn `UserConstructionScript`)